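; AI controller for patrolling guard NPCs that drives patrol and enemy-engagement behavior.
; On BeginPlay it sets up the patrol blackboard and runs the guard behavior tree.
; AI perception writes sensed actors to the enemy key, skipping those tagged "Enemy" so guards ignore each other, and clears it when sensing is lost.
; Each tick, the guard's aiming and shooting flags mirror whether a valid focus actor exists.
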(event `self.ReceiveBeginPlay`
  ;[1 1 1] Creates and Starts AI
  (bind _blackboardcomponent (`self.UseBlackboard` "/Game/Dynamic/NPC/AI/PatrolData.PatrolData"))
  (`self.RunBehaviorTree` "/Game/Dynamic/NPC/AI/GuardBehavior.GuardBehavior")
  (set `self.BlackboardComp` _blackboardcomponent))

(event `self.ReceiveTick`
  (params (DeltaSeconds :type "Float (single-precision)"))
  (bind _returnvalue (`KismetSystemLibrary.IsValid` (`self.GetFocusActor`)))
  ;[1 1 1] Determines Shooting & Aiming States
  (bind _aspatrolling_guard_2 (cast `/Game/Dynamic/NPC/Behavior/PatrollingGuard2` (`self.K2_GetPawn`)))
  (set `/Game/Dynamic/NPC/Behavior/PatrollingGuard2.Aiming` _returnvalue _aspatrolling_guard_2)
  (set `/Game/Dynamic/NPC/Behavior/PatrollingGuard2.Shooting` _returnvalue _aspatrolling_guard_2))

(event `self.AIPerception.OnTargetPerceptionUpdated`
  (params (Actor :type "Actor Object Reference") (Stimulus :type "AIStimulus Structure"))
  (bind _enemykey (`self.EnemyKey`))
  (bind _blackboardcomp (`self.BlackboardComp`))
  ;[1 1 1] Prevents Targeting Other AI
  (if (`self.ActorHasTag` Actor "Enemy")
    _
    (elif (`.bSuccessfullySensed` (break `AIStimulus` Stimulus))
      (`BlackboardComponent.SetValueAsObject` _blackboardcomp _enemykey Actor)
      (else
        (`BlackboardComponent.ClearValue` _blackboardcomp _enemykey)))))

(fn `UserConstructionScript`)